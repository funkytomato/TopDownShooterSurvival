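; Unarmed melee enemy AI that starts asleep and extends a parent enemy class's attack, damage and death events.
; Rising from slumber plays a sound and disables movement for a random delay before marking it ready.
; Attack then faces the shooter character and, within range, moves in to melee, otherwise resumes searching.
; Damage randomly triggers hit reactions; hit and attack montages are picked randomly and gated by DoOnce until their duration elapses.
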(event EventBeginPlay
  (|CallParentFunction)
  (Variables|Default|SetSleeping true)
  (Variables|Default|SetAwakeDuration (Math|Random|RandomFloatinRange 0.2 2.0)))

(event Collision|EventActorBeginOverlap
  (params (OtherActor :type Actor%20Object%20Reference)))

(event EventTick
  (params (DeltaSeconds :type Float%20%28single-precision%29))
  (|CallParentFunction DeltaSeconds) ; This node is disabled and will not be called.\nDrag off pins to build functionality.
)

(fn ConstructionScript
  (|CallParentFunction))

(event Custom|Sleep
  ;[1 1 1] Sleep and Awake
  (Variables|Default|SetSleeping true))

(event Custom|Awake
  ;[1 1 1] Sleep and Awake
  (Variables|Default|SetSleeping false))

(event Custom|RiseUpFromSlomber
  (bind _charactermovement (Variables|Character|GetCharacterMovement))
  (bind _awaking_sound (Variables|Default|GetAwaking%20Sound))
  ;[1 1 1] Sleep and Awake
  (Pawn|Components|CharacterMovement|DisableMovement (Variables|Character|GetCharacterMovement))
  (Audio|PlaySound2D (Utilities|Array|Get(acopy) _awaking_sound (Math|Random|RandomIntegerinRange 0 (- (Utilities|Array|Length _awaking_sound) 1))) 1.0 1.0 0.0 0 0)
  (Utilities|FlowControl|Delay (Variables|Default|GetAwakeDuration))
  (Utilities|IsValid _charactermovement
    (:Is%20Valid
      (Pawn|Components|CharacterMovement|SetMovementMode _charactermovement "MOVE_Walking" 0)
      (Variables|Default|SetIsReadyToMove? true))))

(event Game|Damage|EventAnyDamage
  (params (Damage :type Float%20%28single-precision%29) (DamageType :type Damage%20Type%20Object%20Reference) (InstigatedBy :type Controller%20Object%20Reference) (DamageCauser :type Actor%20Object%20Reference))
  (bind _hitsounds (Variables|Default|GetHitSounds))
  (bind _gethitmontages (Variables|Default|GetGetHitMontages))
  ;[1 1 1] Play Hit Animation randomly
  (|CallParentFunction Damage DamageType InstigatedBy DamageCauser)
  (if (and (Math|Random|RandomBool) (Utilities|IsValid (Variables|Character|GetCharacterMovement)))
    (Utilities|FlowControl|Sequence
      (:then_0
        (Class|NavMovementComponent|StopActiveMovement (Variables|Character|GetCharacterMovement))
        (Utilities|FlowControl|DoOnce false :!label _label
          (:Completed
            (bind _returnvalue (Animation|PlayAnimMontage (Utilities|Array|Get(acopy) _gethitmontages (Math|Random|RandomIntegerinRange 0 (- (Utilities|Array|Length _gethitmontages) 1))) 1.0 "None"))
            (Audio|PlaySound2D (Utilities|Array|Get(acopy) _hitsounds (Math|Random|RandomIntegerinRange 0 (- 0 (Utilities|Array|Length _hitsounds)))) 1.0 1.0 0.0 0 0)
            (Utilities|FlowControl|Delay _returnvalue)
            (goto _label Reset))))
      (:then_1
        ;;[1 1 1] Do I need this???
        (Components|Activation|SetActive (Variables|Character|GetCharacterMovement) true true)))))

(event EventDeathEvent
  ;[1 1 1] Death
  (|CallParentFunction))

(event Custom|PlayAttackAnimation
  (bind _attackmontages (Variables|Default|GetAttackMontages))
  ;[1 1 1] Play Attack Animation
  (Class|NavMovementComponent|StopActiveMovement (Variables|Character|GetCharacterMovement))
  (Utilities|FlowControl|DoOnce false :!label _label
    (:Completed
      (bind _returnvalue (Animation|PlayAnimMontage (Utilities|Array|Get(acopy) _attackmontages (Math|Random|RandomIntegerinRange 0 (- (Utilities|Array|Length _attackmontages) 1))) 1.0 "None"))
      (Utilities|FlowControl|Delay _returnvalue)
      (goto _label Reset))))

(event Custom|Melee
  ;[1 1 1] Melee Attack
  (Variables|Default|SetAttack? true)
  (CallFunction|PlayAttackAnimation))

(event EventAttack
  ;[1 1 1] Override Base Class Attack (This is a Melee Attack)
  (|CallParentFunction)
  ;;[1 1 1] Completed Get up Animation
  (if (Variables|Default|GetIsReadyToMove?)
    (if (not (Variables|Default|GetDeath))
      (Variables|Default|SetAttack? true)
      (Transformation|SetActorRotation (Math|Rotator|MakeRotator 0.0 0.0 (.Yaw (Math|Rotator|BreakRotator (Math|Rotator|FindLookatRotation (Transformation|GetActorLocation) (Transformation|GetActorLocation (Variables|Default|GetShooterCharacter)))))))
      (if (<= (Variables|Default|GetAttackRange) 5e+02)
        (AI|AIMoveTo self "0, 0, 0" (Variables|Default|GetShooterCharacter) 25.0 false
          (:OnSuccess
            (CallFunction|Melee)))
        (else
          (Animation|StopAnimMontage (Animation|GetCurrentMontage :!class /Script/Engine.Character))
          (Variables|Default|SetAttack? false)
          (CallFunction|SearchCharacter))))))