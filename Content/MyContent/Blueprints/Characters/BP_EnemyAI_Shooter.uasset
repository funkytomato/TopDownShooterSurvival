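; BP_EnemyAI_Shooter is a ranged enemy character that fires projectiles at the player and carries a gun snapped to its WeaponSocket.
; On BeginPlay, after a short delay, it shows or hides its flashlight based on Night.
; Attack checks death, range and reload state, stops and yaws toward the player, then spawns BP_EnemyProjectile from Arrow1, reloads when empty or searches.
; Threatened is empty, with its under-fire and behavior tree logic left disconnected.
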(event Custom|Threatened
  (params (ThreatSource :type Vector))
  ;[1 1 1] Threatened
)

(event Custom|Night?
  (bind _flashlight (Variables|Default|GetFlashlight))
  ;[1 1 1] IfNightTrue - Flashlight On
  (if (Variables|Default|GetNight)
    (Rendering|SetVisibility _flashlight true false)
    (else
      (Rendering|SetVisibility _flashlight false false))))

(event EventBeginPlay
  ;[1 1 1] OnBeginPlay - If Nightm turn on Flashlight
  (|CallParentFunction)
  (Utilities|FlowControl|Delay 0.2)
  (CallFunction|Night?))

(event Collision|EventActorBeginOverlap
  (params (OtherActor :type Actor%20Object%20Reference)))

(event EventTick
  (params (DeltaSeconds :type Float%20%28single-precision%29))
  (|CallParentFunction DeltaSeconds) ; This node is disabled and will not be called.\nDrag off pins to build functionality.
)

(event EventAttack
  (bind _arrow1 (Variables|Default|GetArrow1))
  (bind _returnvalue (Transformation|GetWorldRotation _arrow1))
  ;[1 1 1] Shooter Attack
  (if (not (Variables|Default|GetDeath))
    (if (Variables|Default|GetInRange)
      (if (not (Variables|Default|GetReloading))
        (Variables|Default|SetAttack? true)
        (Components|Movement|StopMovementImmediately (Variables|Character|GetCharacterMovement))
        (Transformation|SetActorRotation (Math|Rotator|MakeRotator 0.0 0.0 (.Yaw (Math|Rotator|BreakRotator (Math|Rotator|FindLookatRotation (Transformation|GetActorLocation) (Transformation|GetActorLocation (Variables|Default|GetShooterCharacter)))))))
        (if (<= (Variables|Default|GetAttackRange) (Variables|Default|GetMaxDetectionRange))
          (if (>= (Variables|Default|GetAmmo) 1)
            (Variables|Default|SetAmmo (- (Variables|Default|GetAmmo) 1))
            (Game|SpawnActorfromClass "/Game/MyContent/Blueprints/Projectiles/BP_EnemyProjectile.BP_EnemyProjectile_C" (Math|Transform|MakeTransform (+ (Transformation|GetWorldLocation (Variables|Default|GetArrow1)) (Math|Vector|RotateVector (Variables|Default|GetGunOfset) _returnvalue)) _returnvalue) "Undefined" 0 0)
            (Audio|Components|Audio|Play (Variables|Default|GetAttackAudio) 0.0)
            (else
              (CallFunction|Reload)))
          (else
            (CallFunction|SearchCharacter)))))))

(fn ConstructionScript
  (|CallParentFunction)
  (Transformation|AttachComponentToComponent (Variables|Default|GetSK_FPGun2) (Variables|Character|GetMesh) "WeaponSocket" "SnapToTarget" "SnapToTarget" "SnapToTarget" true))