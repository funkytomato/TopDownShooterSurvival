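; Master enemy AI character for a top-down shooter, driven by pawn sensing and AI MoveTo.
; Sensing triggers chasing, but the player-attack logic is disconnected and melee is empty; only slow or stopped occupied cars get shot.
; Fast cars make it flee or kill it on overlap.
; Tick polls health for death, handling animations, ragdoll for car kills, player XP and random slow-motion kill cams, alongside burn damage, reloading and blood effects.
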(event Custom|Fire%20Projectile
  (bind _arrow1 (Variables|Default|GetArrow1))
  (bind _returnvalue (Transformation|GetWorldRotation _arrow1))
  ;[1 1 1] Fire Projectile
  (if (>= (Variables|Weapon|GetAmmo) 1)
    (Variables|Weapon|SetAmmo (- (Variables|Weapon|GetAmmo) 1))
    (Game|SpawnActorfromClass "/Game/MyContent/Blueprints/Projectiles/BP_EnemyProjectile.BP_EnemyProjectile_C" (Math|Transform|MakeTransform (+ (Transformation|GetWorldLocation (Variables|Default|GetArrow1)) (Math|Vector|RotateVector (Variables|Weapon|GetGunOfset) _returnvalue)) _returnvalue) "Undefined" 0 0)
    (Audio|Components|Audio|Play (Variables|Default|GetAttackAudio) 0.0)
    (else
      (CallFunction|Reload))))

(event Custom|Attack
  ;[1 1 1] If the enemy sees the player and is not dead, does not recharge, then he will attack the player if the distance is less than 500 units. If there are no ammo it is recharged.
)

(event Custom|Melee
  ;[1 1 1] Melee
)

(event EventTick
  (params (DeltaSeconds :type Float%20%28single-precision%29))
  ;[1 1 1] Event Tick Checking Death of Enemy
  (CallFunction|DeathEvent))

(event EventBeginPlay
  ;[1 1 1] Event Begin Play\set Initial Location
  (bind _asbp_tds_character (Utilities|Casting|CastToBP_TDS_Character (Game|GetPlayerCharacter 0)))
  (Variables|EnemyDetection|SetShooterCharacter _asbp_tds_character)
  (Variables|Character|SetInitialLocation (Transformation|GetActorLocation))
  (Components|Activation|Deactivate (Variables|Default|GetCharacterOnFireEmitter)))

(fn ConstructionScript)

(event OnComponentBeginOverlap(Capsule)
  (params (OverlappedComponent :type Primitive%20Component%20Object%20Reference) (OtherActor :type Actor%20Object%20Reference) (OtherComp :type Primitive%20Component%20Object%20Reference) (OtherBodyIndex :type Integer) (bFromSweep :type Boolean) (SweepResult :type Hit%20Result%20Structure%20%28by%20ref%29))
  ;[1 1 1 1 20] In-Car Events
  ;;[1 1 1] Car Hit Event
  (bind _asbp_sedan (Utilities|Casting|CastToBP_Sedan OtherActor))
  (Utilities|IsValid (Variables|/Script/PhysXVehicles.WheeledVehicle|GetVehicleMovement _asbp_sedan)
    (:Is%20Valid
      (if (or (>= (Class|WheeledVehicleMovementComponent|GetForwardSpeed (Variables|/Script/PhysXVehicles.WheeledVehicle|GetVehicleMovement _asbp_sedan)) 5e+02) (<= (Class|WheeledVehicleMovementComponent|GetForwardSpeed (Variables|/Script/PhysXVehicles.WheeledVehicle|GetVehicleMovement _asbp_sedan)) -5e+02))
        (Variables|Character|SetHealth 0.0)
        (Variables|Character|SetDeathByCar true)
        (Audio|Components|Audio|Play (Variables|Default|GetHit) 0.0)))))

(event OnSeePawn(PawnSensing1)
  (params (Pawn :type Pawn%20Object%20Reference))
  ;[1 1 1 1 20] In-Car Events
  ;;[1 1 1] If a car with a character inside moves fast, the enemy escapes to a random point. Upon reaching it, he returns to the initial location.
  (bind _asbp_sedan (Utilities|Casting|CastToBP_Sedan Pawn))
  (Utilities|IsValid (Variables|/Script/PhysXVehicles.WheeledVehicle|GetVehicleMovement _asbp_sedan)
    (:Is%20Valid
      (if (or (>= (Class|WheeledVehicleMovementComponent|GetForwardSpeed (Variables|/Script/PhysXVehicles.WheeledVehicle|GetVehicleMovement _asbp_sedan)) 5e+02) (<= (Class|WheeledVehicleMovementComponent|GetForwardSpeed (Variables|/Script/PhysXVehicles.WheeledVehicle|GetVehicleMovement _asbp_sedan)) -5e+02))
        (AI|AIMoveTo self (.RandomLocation (Class|NavigationSystemV1|GetRandomPointinNavigableRadius (Transformation|GetActorLocation _asbp_sedan) 6e+03 0 0)) 0 5.0 false
          (:OnSuccess
            (Utilities|FlowControl|Delay 3.0)
            (AI|AIMoveTo self (Variables|Character|GetInitialLocation) 0 5.0 false)))
        (elif (Variables|/Game/MyContent/Blueprints/Vehicles/BP_Sedan.BP_Sedan_C|GetInCar _asbp_sedan)
          (CallFunction|AttackCar))))))

(event Custom|Reload
  ;[1 1 1] Reloading
  (if (< (Variables|Weapon|GetAmmo) 8)
    (if (not (Variables|Character|GetDeath))
      (Components|Animation|PlayAnimation (Variables|Character|GetMesh) "/Game/MyContent/ExampleContent/AnimStarterPack/Reload_Shotgun_Hip.Reload_Shotgun_Hip" false)
      (Variables|Weapon|SetReloading true)
      (if (>= (Variables|Weapon|GetMaxAmmo) 0)
        (Variables|Weapon|SetNeedAmmo (- (Variables|Weapon|GetMaxAmmo) 8))
        (if (<= (Variables|Weapon|GetMaxAmmo) (Variables|Weapon|GetNeedAmmo))
          (Variables|Weapon|SetAmmo (+ (Variables|Weapon|GetAmmo) (Variables|Weapon|GetMaxAmmo)))
          (Variables|Weapon|SetMaxAmmo 0)
          (else
            (Variables|Weapon|SetMaxAmmo (- (Variables|Weapon|GetMaxAmmo) (Variables|Weapon|GetNeedAmmo)))
            (Variables|Weapon|SetAmmo 8)))
        (Utilities|FlowControl|Delay 4.3)
        (Variables|Weapon|SetReloading false)
        (if (not (Variables|Character|GetDeath))
          (Components|Animation|SetAnimationMode (Variables|Character|GetMesh) "AnimationBlueprint"))))))

(event Custom|AttackCar
  (bind _arrow1 (Variables|Default|GetArrow1))
  (bind _returnvalue (Transformation|GetWorldRotation _arrow1))
  ;[1 1 1 1 20] In-Car Events
  ;;[1 1 1] If the car is standing with the character inside or moving slowly, the enemy attacks the car, causing damage to it.
  (if (not (Variables|Character|GetDeath))
    (if (not (Variables|Weapon|GetReloading))
      (Variables|EnemyDetection|SetAttack? true)
      (Components|Movement|StopMovementImmediately (Variables|Character|GetCharacterMovement))
      (Transformation|SetActorRotation (Math|Rotator|MakeRotator 0.0 0.0 (.Yaw (Math|Rotator|BreakRotator (Math|Rotator|FindLookatRotation (Transformation|GetActorLocation) (Transformation|GetActorLocation (stale OnSeePawn(PawnSensing1) _asbp_sedan)))))))
      (if (<= (Variables|EnemyDetection|GetAttackRange) 5e+02)
        (if (>= (Variables|Weapon|GetAmmo) 1)
          (Variables|Weapon|SetAmmo (- (Variables|Weapon|GetAmmo) 1))
          (Game|SpawnActorfromClass "/Game/MyContent/Blueprints/Projectiles/BP_EnemyProjectile.BP_EnemyProjectile_C" (Math|Transform|MakeTransform (+ (Transformation|GetWorldLocation (Variables|Default|GetArrow1)) (Math|Vector|RotateVector (Variables|Weapon|GetGunOfset) _returnvalue)) _returnvalue) "Undefined" 0 0)
          (Audio|Components|Audio|Play (Variables|Default|GetAttackAudio) 0.0)
          (else
            (CallFunction|Reload)))
        (else
          (CallFunction|SearchCharacter))))))

(event Custom|OnFireEvent
  (params (DamageCauser :type Actor%20Object%20Reference))
  ;[1 1 1] On Fire Events
  (Variables|Character|SetOnFire true)
  (Components|Activation|Activate (Variables|Default|GetCharacterOnFireEmitter) false)
  (bind _returnvalue (Utilities|Time|SetTimerbyEvent (delegate Custom|FireDamage) 1.0 true))
  (Variables|Default|SetFireDamageTimer _returnvalue))

(event Custom|PlayFireDeathAnimation
  (bind _onfireanimseqs (Variables|Animations|GetOnFireAnimSeqs))
  ;[1 1 1] On Fire Events
  (Components|Animation|PlayAnimation (Variables|Character|GetMesh) (Utilities|Array|Get(acopy) _onfireanimseqs (Math|Random|RandomIntegerinRange 0 (- (Utilities|Array|Length _onfireanimseqs) 1))) false)
  ;;[1 1 1] Clear Fire Damage Timer
  (Utilities|Time|ClearandInvalidateTimerbyHandle (Variables|Default|GetFireDamageTimer)))

(event Custom|FireDamage
  ;[1 1 1] On Fire Events
  ;;[1 1 1] Fire Damage whilst burning
  (bind _returnvalue (Game|Damage|ApplyDamage self 1e+01 (Game|GetPlayerController 0) (stale Custom|OnFireEvent DamageCauser)))
  (Development|PrintString (Utilities|String|ToString(Text) (Utilities|Text|FormatText "{a} on fire damage {b}" self _returnvalue))))

(event Custom|DeathEvent
  (bind _shootercharacter (Variables|EnemyDetection|GetShooterCharacter))
  (bind _capsule (Variables|Default|GetCapsule))
  ;[1 1 1] if health is zero or less, the “Dead” variable becomes true, animation plays, components are destroyed, other components are given a static type of collision so that they can no longer be shot at.
  (if (<= (Variables|Character|GetHealth) 0.0)
    (Variables|Character|SetDeath true)
    (Utilities|FlowControl|DoOnce false
      (:Completed
        (if (Variables|Character|GetOnFire)
          (CallFunction|PlayFireDeathAnimation)
          (else
            (CallFunction|PlayDeathAnnimation)))
        (CallFunction|PlayDeathSound)
        (Components|DestroyComponent (Variables|Character|GetCharacterMovement))
        (Collision|SetCollisionObjectType (Variables|Collision|GetCapsuleComponent) "ECC_WorldStatic")
        (Utilities|IsValid _capsule
          (:Is%20Valid
            (Components|DestroyComponent _capsule)
            (if (Variables|Character|GetDeathByCar)
              (Physics|SetSimulatePhysics (Variables|Character|GetMesh) true)
              (else
                ;;[1 1 1] WhenCharacterKillTheEnemies - + XP
                (Utilities|IsValid _shootercharacter
                  (:Is%20Valid
                    (Variables|/Game/MyContent/Blueprints/Characters/BP_TDS_Character.BP_TDS_Character_C|SetXP _shootercharacter (+ (Variables|/Game/MyContent/Blueprints/Characters/BP_TDS_Character.BP_TDS_Character_C|GetXP _shootercharacter) 100))
                    (bind _foundwidgets (Widget|GetAllWidgetsOfClass "/Game/MyContent/Widgets/BP_HUD_Widget.BP_HUD_Widget_C" false))
                    (for _array_element _foundwidgets
                      (UserInterface|Animation|PlayAnimation _array_element (Variables|/Game/MyContent/Widgets/BP_HUD_Widget.BP_HUD_Widget_C|GetXP_TextAnim _array_element) 0.0 1 "Forward" 1.0 false)
                      ;;[1 1 1] SlowMoEvent
                      (if (== (Math|Random|RandomIntegerinRange 0 4) 4)
                        (Variables|VisualEffects|SetSlowMo true)
                        (Utilities|Time|SetGlobalTimeDilation 0.1)
                        (Audio|Components|Audio|Play (Variables|Default|Getaiming_reverse_wav_Cue) 0.0)
                        (Game|Player|SetViewTargetwithBlend (Game|GetPlayerController 0) self 0.1 "VTBlend_Linear" 0.0 false)
                        (Utilities|FlowControl|Delay 0.2)
                        (Game|Player|SetViewTargetwithBlend (Game|GetPlayerController 0) (Game|GetPlayerCharacter 0) 0.1 "VTBlend_Linear" 0.0 false)
                        (Audio|Components|Audio|Play (Variables|Default|Getreverese_Cue) 0.0)
                        (Utilities|Time|SetGlobalTimeDilation 1.0)
                        (Audio|Components|Audio|SetPitchMultiplier (Variables|Default|GetAttackAudio) 1.0)
                        (for _array_element_2 0
                          (Audio|Components|Audio|SetPitchMultiplier (Variables|/Script/Engine.AmbientSound|GetAudioComponent _array_element_2) 1.0)
                          (Variables|VisualEffects|SetSlowMo false))))))))))))))

(event Custom|PlayHitSounds
  (bind _hitsounds (Variables|SoundEffects|GetHitSounds))
  ;[1 1 1] Sound Effects
  ;;[1 1 1] Play Hit SFX
  (if (Math|Random|RandomBool)
    (Audio|PlaySound2D (Utilities|Array|Get(acopy) _hitsounds (Math|Random|RandomIntegerinRange 0 (- (Utilities|Array|Length _hitsounds) 1))) 1.0 1.0 0.0 0 0)))

(event Custom|PlayAttackSounds
  (bind _attacksounds (Variables|SoundEffects|GetAttackSounds))
  ;[1 1 1] Sound Effects
  ;;[1 1 1] Play Attack SFX
  (if (Math|Random|RandomBool)
    (Audio|PlaySound2D (Utilities|Array|Get(acopy) _attacksounds (Math|Random|RandomIntegerinRange 0 (- (Utilities|Array|Length _attacksounds) 1))) 1.0 1.0 0.0 0 0)))

(event Custom|PlayDeathAnnimation
  (bind _deathanimseqs (Variables|Animations|GetDeathAnimSeqs))
  ;[1 1 1] Play Death Animation
  (Components|Animation|PlayAnimation (Variables|Character|GetMesh) (Utilities|Array|Get(acopy) _deathanimseqs (Math|Random|RandomIntegerinRange 0 (- (Utilities|Array|Length _deathanimseqs) 1))) false))

(event Custom|ApplyDamageFX
  (bind _bloodspurtfx (Variables|VisualEffects|GetBloodSpurtFX))
  ;[1 1 1] Apply Damage FX
  (Effects|SpawnEmitterAttached (Utilities|Array|Get(acopy) _bloodspurtfx (Math|Random|RandomIntegerinRange 0 (Utilities|Array|Length _bloodspurtfx))) (Variables|Character|GetMesh) "None" "0, 0, 0" (Math|Random|RandomRotator false) "2.000000,2.000000,2.000000" "SnapToTarget" true "AutoRelease")
  (if (Math|Random|RandomBool)
    (bind _output_get (Variables|VisualEffects|SetDecalScale (Math|Random|RandomFloatinRange 5e+01 2.5e+02)))
    (Rendering|Decal|SpawnDecalatLocation "/Game/BallisticsVFX/Decals/Splashers/Decal_Blood_Splatter.Decal_Blood_Splatter" (Math|Vector|MakeVector _output_get _output_get _output_get) (Transformation|GetWorldLocation (Variables|Collision|GetCapsuleComponent)) (Math|Random|RandomRotator false) 0.0)))

(event Custom|PlayDeathSound
  (bind _deathsounds (Variables|SoundEffects|GetDeathSounds))
  ;[1 1 1] Sound Effects
  ;;[1 1 1] Play Death SFX
  (if (Math|Random|RandomBool)
    (Audio|PlaySound2D (Utilities|Array|Get(acopy) _deathsounds (Math|Random|RandomIntegerinRange 0 (- (Utilities|Array|Length _deathsounds) 1))) 1.0 1.0 0.0 0 0)))

(event Game|Damage|EventAnyDamage
  (params (Damage :type Float%20%28single-precision%29) (DamageType :type Damage%20Type%20Object%20Reference) (InstigatedBy :type Controller%20Object%20Reference) (DamageCauser :type Actor%20Object%20Reference))
  ;[1 1 1] When receiving damage the enemy loses health corresponding to damage.
  (Variables|Character|SetHealth (- (Variables|Character|GetHealth) Damage))
  (Transformation|SetActorRotation (Math|Rotator|MakeRotator 0.0 0.0 (.Yaw (Math|Rotator|BreakRotator (Math|Rotator|FindLookatRotation (Transformation|GetActorLocation) (Transformation|GetActorLocation (Variables|EnemyDetection|GetShooterCharacter)))))))
  ;;[1 1 1] No Damage FX if burning
  (if (not (Variables|Character|GetOnFire))
    (CallFunction|ApplyDamageFX)))

(event OnSeePawn(PawnSensing)
  (params (Pawn :type Pawn%20Object%20Reference))
  ;[1 1 1] When an enemy sees, or hears, a player, he will attack him. If he saw, or heard the enemy, but lost him from sight, then the enemy, after a pause, begins to look for a player
  (bind _asbp_tds_character (Utilities|Casting|CastToBP_TDS_Character Pawn))
  (if (not (Variables|/Game/MyContent/Blueprints/Characters/BP_TDS_Character.BP_TDS_Character_C|GetDead _asbp_tds_character))
    (if (not (Variables|Character|GetDeath))
      (Variables|Character|SetSleeping false)
      (Variables|EnemyDetection|SetInRange true)
      (Variables|EnemyDetection|SetSeePlayer true)
      (CallFunction|Attack)
      (Utilities|FlowControl|Delay 1.0)
      (Variables|EnemyDetection|SetInRange false)
      (if (Variables|EnemyDetection|GetSeePlayer)
        (Utilities|FlowControl|Delay 5.0)
        (if (not (Variables|EnemyDetection|GetInRange))
          (CallFunction|SearchCharacter))))))

(event OnHearNoise(PawnSensing)
  (params (Instigator :type Pawn%20Object%20Reference) (Location :type Vector%20%28by%20ref%29 :default "0, 0, 0") (Volume :type Float%20%28single-precision%29))
  ;[1 1 1] When an enemy sees, or hears, a player, he will attack him. If he saw, or heard the enemy, but lost him from sight, then the enemy, after a pause, begins to look for a player
  (if (not (Variables|Character|GetDeath))
    (Variables|Character|SetSleeping false)
    (Variables|EnemyDetection|SetInRange true)
    (Variables|EnemyDetection|SetSeePlayer true)
    (CallFunction|Attack)
    (Utilities|FlowControl|Delay 1.0)
    (Variables|EnemyDetection|SetInRange false)
    (if (Variables|EnemyDetection|GetSeePlayer)
      (Utilities|FlowControl|Delay 5.0)
      (if (not (Variables|EnemyDetection|GetInRange))
        (CallFunction|SearchCharacter)))))

(event Custom|SearchCharacter
  (bind _returnvalue (Game|GetPlayerCharacter 0))
  ;[1 1 1] Player search. With success = attack.
  (if (Variables|Default|GetIsReadyToMove?)
    (if (not (Variables|Character|GetDeath))
      (if (not (Variables|Weapon|GetReloading))
        (Utilities|IsValid _returnvalue
          (:Is%20Valid
            (Variables|EnemyDetection|SetAttackRange (Math|Vector|VectorLength (- (Transformation|GetActorLocation) (Transformation|GetActorLocation _returnvalue))))
            (AI|AIMoveTo self (+ (Transformation|GetActorLocation) "500.000000,500.000000,0.000000") (Variables|EnemyDetection|GetShooterCharacter) 5.0 false
              (:then
                (if (<= (Variables|EnemyDetection|GetAttackRange) 5e+02)
                  (CallFunction|Attack))))))))))