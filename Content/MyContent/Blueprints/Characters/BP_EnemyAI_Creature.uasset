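; BP_EnemyAI_Creature is an enemy AI creature that extends its parent's attack and death behavior and can dodge incoming projectiles.
; Attacking runs the parent logic, then calls Awake.
; When a BP_CharacterProjectile enters its evade sphere, a coin flip decides whether it stops movement and evades, and a second flip sets either the EvadeLeft or EvadeRight flag.
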(event OnComponentBeginOverlap(EvadeSphereCollision)
  (params (OverlappedComponent :type Primitive%20Component%20Object%20Reference) (OtherActor :type Actor%20Object%20Reference) (OtherComp :type Primitive%20Component%20Object%20Reference) (OtherBodyIndex :type Integer) (bFromSweep :type Boolean) (SweepResult :type Hit%20Result%20Structure%20%28by%20ref%29))
  ;[1 1 1] Evade Incoming Projectiles
  ;;[1 1 1] If under fire, attempt evasion of projectiles
  (Utilities|Casting|CastToBP_CharacterProjectile OtherActor)
  (CallFunction|Evade))

(event Custom|Evade
  ;[1 1 1] Evade Incoming Projectiles
  ;;[1 1 1] Evade
  (Utilities|IsValid (Variables|Character|GetCharacterMovement)
    (:Is%20Valid
      ;;;[1 1 1] Randomise Evasion Attempt
      (if (Math|Random|RandomBool)
        (Components|Movement|StopMovementImmediately (Variables|Character|GetCharacterMovement))
        ;;;[1 1 1] Randomise Direction
        (if (Math|Random|RandomBool)
          (Variables|Default|SetEvadeLeft true)
          (else
            (Variables|Default|SetEvadeRight true)))))))

(event EventBeginPlay
  (|CallParentFunction))

(event Collision|EventActorBeginOverlap
  (params (OtherActor :type Actor%20Object%20Reference))
  (|CallParentFunction OtherActor) ; This node is disabled and will not be called.\nDrag off pins to build functionality.
)

(event EventTick
  (params (DeltaSeconds :type Float%20%28single-precision%29))
  (|CallParentFunction DeltaSeconds) ; This node is disabled and will not be called.\nDrag off pins to build functionality.
)

(event EventAttack
  ;[1 1 1] Attack
  (|CallParentFunction)
  (CallFunction|Awake))

(event EventDeathEvent
  ;[1 1 1] Death
  (|CallParentFunction))

(fn ConstructionScript
  (|CallParentFunction))