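; Blue ammo pickup actor that adds reserve ammo to the player's gun on overlap.
; Box overlap casts to BP_TDS_Character and raises the equipped gun's GunAmmoMax by a fixed amount, without checking the gun type.
; It then plays PickUpCue, creates a new BP_Ammo_Widget on the viewport and removes the box, text and rune components.
; The actor destroys itself after a short delay.
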(event OnComponentBeginOverlap(Box)
  (params (OverlappedComponent :type Primitive%20Component%20Object%20Reference) (OtherActor :type Actor%20Object%20Reference) (OtherComp :type Primitive%20Component%20Object%20Reference) (OtherBodyIndex :type Integer) (bFromSweep :type Boolean) (SweepResult :type Hit%20Result%20Structure%20%28by%20ref%29))
  ;[1 1 1] Pick Up Ammo for Blue Gun
  (bind _asbp_tds_character (Utilities|Casting|CastToBP_TDS_Character OtherActor))
  (Variables|/Game/MyContent/Blueprints/Weapons/BP_MasterGun.BP_MasterGun_C|SetGunAmmoMax (Variables|/Game/MyContent/Blueprints/Characters/BP_TDS_Character.BP_TDS_Character_C|GetEquippedGun _asbp_tds_character) (+ (Variables|/Game/MyContent/Blueprints/Weapons/BP_MasterGun.BP_MasterGun_C|GetGunAmmoMax (Variables|/Game/MyContent/Blueprints/Characters/BP_TDS_Character.BP_TDS_Character_C|GetEquippedGun _asbp_tds_character)) 100))
  (Audio|Components|Audio|Play (Variables|Default|GetPickUp_Cue) 0.0)
  (Components|DestroyComponent (Variables|Default|GetBox))
  (bind _returnvalue (UserInterface|CreateWidget "/Game/MyContent/Widgets/BP_+Ammo_Widget.BP_+Ammo_Widget_C"))
  (UserInterface|Viewport|AddtoViewport _returnvalue 0)
  (Components|DestroyComponent (Variables|Default|GetRune_P2))
  (Utilities|FlowControl|Delay 1.0)
  (Actor|DestroyActor))

(fn ConstructionScript)