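; Base gun actor for the top-down shooter, which takes its parent actor, a BP_TDS_Character, as GunOwner.
; TriggerPressed and Reloading are empty; TriggerReleased closes a gate whose repeating ammo-decrement loop has its start logic disconnected.
; ThreatTrace runs a zero-length sphere trace at the muzzle, sized by ThreatValue, and calls Threatened on a hit character or shooter AI, depending on the owner's class.
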(event Custom|Reloading)

(event Custom|TriggerPressed)

(event Custom|Trigger%20Released
  (Utilities|FlowControl|Gate true) ; enters at Close
)

(event EventBeginPlay
  (bind _asbp_tds_character (Utilities|Casting|CastToBP_TDS_Character (Actor|GetParentActor)))
  (Variables|Default|SetGunOwner _asbp_tds_character))

(event Collision|EventActorBeginOverlap
  (params (OtherActor :type Actor%20Object%20Reference)))

(fn ConstructionScript)

(fn ThreatTrace
  (params (ThreatValue :type Float%20%28single-precision%29))
  (bind _muzzle_ref (Variables|Default|GetMuzzle%20Ref))
  (bind _returnvalue (Transformation|GetWorldLocation _muzzle_ref))
  ;[1 1 1] ast
  (bind _asbp_tds_character (Utilities|Casting|CastToBP_TDS_Character (Variables|Default|GetGunOwner)))
  (bind _outhit (Collision|SphereTraceByChannel _returnvalue (+ _returnvalue (* (Math|Vector|GetForwardVector (Transformation|GetWorldRotation (Variables|/Game/MyContent/Blueprints/Characters/BP_TDS_Character.BP_TDS_Character_C|GetArrow2 _asbp_tds_character))) 0.0)) ThreatValue "TraceTypeQuery2" false (Utilities|Array|MakeArray 0) "None" true "(R=0.009268,G=0.021773,B=1.000000,A=1.000000)" "(R=0.000000,G=0.795357,B=1.000000,A=1.000000)"))
  (if (.bblockinghit _outhit)
    (bind _asbp_tds_character_2 (Utilities|Casting|CastToBP_TDS_Character (.hitactor _outhit))
      (:then
        (Utilities|Casting|CastToBP_EnemyAI_Shooter (Variables|Default|GetGunOwner))
        (Default|Threatened _asbp_tds_character_2))
      (:CastFailed
        (bind _asbp_enemy_ai_shooter (Utilities|Casting|CastToBP_EnemyAI_Shooter (.hitactor _outhit)))
        (Utilities|Casting|CastToBP_TDS_Character (Variables|Default|GetGunOwner))
        (Default|Threatened _asbp_enemy_ai_shooter (.tracestart _outhit))))))