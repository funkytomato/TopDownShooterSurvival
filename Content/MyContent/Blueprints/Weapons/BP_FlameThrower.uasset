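; Flamethrower weapon for the top-down shooter character that sets enemies inside its cone on fire.
; While the trigger is held, a gate and retriggerable-delay loop burns ammo, runs fire effects and emits AI noise.
; Cone overlaps maintain the enemy list, and both that loop and a looping timer call OnFireEvent on each target while firing.
; Reloading refills the clip from reserve ammo, animates ammo widgets and blocks firing briefly.
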(event OnComponentBeginOverlap(Cone)
  (params (OverlappedComponent :type Primitive%20Component%20Object%20Reference) (OtherActor :type Actor%20Object%20Reference) (OtherComp :type Primitive%20Component%20Object%20Reference) (OtherBodyIndex :type Integer) (bFromSweep :type Boolean) (SweepResult :type Hit%20Result%20Structure%20%28by%20ref%29))
  ;[1 1 1] Manage Enemies Within Cone of Death
  (bind _asbp_enemy_ai_master (Utilities|Casting|CastToBP_EnemyAI_Master OtherActor))
  (Utilities|Array|AddUnique (Variables|Default|GetTargetsInCone) _asbp_enemy_ai_master)
  (Development|PrintString (Utilities|String|ToString(Text) (Utilities|Text|FormatText "{a} add to targetsincone" _asbp_enemy_ai_master))))

(event OnComponentEndOverlap(Cone)
  (params (OverlappedComponent :type Primitive%20Component%20Object%20Reference) (OtherActor :type Actor%20Object%20Reference) (OtherComp :type Primitive%20Component%20Object%20Reference) (OtherBodyIndex :type Integer))
  ;[1 1 1] Manage Enemies Within Cone of Death
  (bind _asbp_enemy_ai_master (Utilities|Casting|CastToBP_EnemyAI_Master OtherActor))
  (Utilities|Array|RemoveItem (Variables|Default|GetTargetsInCone) _asbp_enemy_ai_master)
  (Development|PrintString (Utilities|String|ToString(Text) (Utilities|Text|FormatText "{a} add to targetsincone" _asbp_enemy_ai_master))))

(event Custom|ApplyFlameDamage
  ;[1 1 1] Apply Flame Damage
  (if (Variables|Default|GetIsTriggered?)
    (for _array_element (Variables|Default|GetTargetsInCone)
      (Development|PrintString (Utilities|String|ToString(Text) (Utilities|Text|FormatText "{a} is on fire" _array_element)))
      (Default|OnFireEvent _array_element self))))

(event EventBeginPlay
  (|CallParentFunction)
  (bind _returnvalue (Utilities|Time|SetTimerbyFunctionName self "ApplyFlameDamage" 0.1 true))
  (Variables|Default|SetFlameDamageTimer _returnvalue))

(event Collision|EventActorBeginOverlap
  (params (OtherActor :type Actor%20Object%20Reference))
  (|CallParentFunction OtherActor) ; This node is disabled and will not be called.\nDrag off pins to build functionality.
)

(event EventTriggerPressed
  (bind _firesfx (Variables|Default|GetFireSFX))
  ;[1 1 1] Trigger Pressed
  (|CallParentFunction)
  (if (not (Variables|Default|GetReload))
    (bind _asbp_tds_character (Utilities|Casting|CastToBP_TDS_Character (Variables|Default|GetGunOwner)))
    (if (Variables|/Game/MyContent/Blueprints/Characters/BP_TDS_Character.BP_TDS_Character_C|GetUseGun _asbp_tds_character)
      (Utilities|FlowControl|Sequence
        (:then_0
          (goto _label Open))
        (:then_1
          (Utilities|FlowControl|Gate true :!label _label
            (:Exit
              (Utilities|FlowControl|Sequence
                (:then_0
                  (Utilities|FlowControl|RetriggerableDelay 0.1)
                  (goto _label))
                (:then_1
                  (if (>= (Variables|Default|GetGunAmmo) 1)
                    (Variables|Default|SetGunAmmo (- (Variables|Default|GetGunAmmo) 1))
                    (Variables|Default|SetIsTriggered? true)
                    (Components|Activation|Activate (Variables|Default|GetFireEmitter) true)
                    (if (Audio|Components|Audio|IsPlaying _firesfx)
                      _
                      (else
                        (Audio|Components|Audio|Play _firesfx 0.0)))
                    (bind _asbp_tds_character_2 (Utilities|Casting|CastToBP_TDS_Character (Variables|Default|GetGunOwner)))
                    (Class|PawnNoiseEmitterComponent|MakeNoise (Variables|/Game/MyContent/Blueprints/Characters/BP_TDS_Character.BP_TDS_Character_C|GetPawnNoiseEmitter _asbp_tds_character_2) self 1.0 (Transformation|GetActorLocation))
                    (CallFunction|ApplyFlameDamage)
                    (else
                      (Components|Activation|Deactivate (Variables|Default|GetFireEmitter))
                      (Variables|Default|SetIsTriggered? false))))))))))))

(event EventTick
  (params (DeltaSeconds :type Float%20%28single-precision%29)))

(event EventTriggerReleased
  (bind _firesfx (Variables|Default|GetFireSFX))
  ;[1 1 1] Trigger Pressed
  (|CallParentFunction)
  (Variables|Default|SetIsTriggered? false)
  (Components|Activation|Deactivate (Variables|Default|GetFireEmitter))
  (Utilities|FlowControl|Gate true) ; enters at Close
)

(event EventReloading
  ;[1 1 1] Reloading
  (|CallParentFunction)
  (bind _asbp_tds_character (Utilities|Casting|CastToBP_TDS_Character (Variables|Default|GetGunOwner)))
  (if (Variables|/Game/MyContent/Blueprints/Characters/BP_TDS_Character.BP_TDS_Character_C|GetUseGun _asbp_tds_character)
    (if (>= (Variables|Default|GetGunAmmoMax) 1)
      (Variables|Default|SetNeedAmmo (- (Variables|Default|GetAmmoClip) (Variables|Default|GetGunAmmo)))
      (if (<= (Variables|Default|GetGunAmmoMax) (Variables|Default|GetNeedAmmo))
        (Variables|Default|SetGunAmmo (+ (Variables|Default|GetGunAmmo) (Variables|Default|GetGunAmmoMax)))
        (Variables|Default|SetGunAmmoMax 0)
        (else
          (Variables|Default|SetGunAmmoMax (- (Variables|Default|GetGunAmmoMax) (Variables|Default|GetNeedAmmo)))
          (Variables|Default|SetGunAmmo 30)))
      (Variables|Default|SetReload true)
      (Audio|Components|Audio|Play (Variables|Default|GetReloadSFX) 0.0)
      (bind _foundwidgets (Widget|GetAllWidgetsOfClass "/Game/MyContent/Widgets/BP_GunAmmoWidget.BP_GunAmmoWidget_C" false))
      (for _array_element _foundwidgets
        (Class|UserWidget|PlayAnimationForward _array_element (Variables|/Game/MyContent/Widgets/BP_GunAmmoWidget.BP_GunAmmoWidget_C|GetButtonAnim _array_element) 1.0 false)
        (Class|UserWidget|PlayAnimationForward _array_element (Variables|/Game/MyContent/Widgets/BP_GunAmmoWidget.BP_GunAmmoWidget_C|GetTextAnim _array_element) 1.0 false)
        (Class|UserWidget|PlayAnimationForward _array_element (Variables|/Game/MyContent/Widgets/BP_GunAmmoWidget.BP_GunAmmoWidget_C|GetTextAnimation _array_element) 1.0 false)
        (Utilities|FlowControl|Delay 1.0)
        (Variables|Default|SetReload false)))))

(fn ConstructionScript
  (|CallParentFunction))