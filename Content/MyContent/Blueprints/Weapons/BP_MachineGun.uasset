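; Machine gun weapon Blueprint that fires projectiles for a BP_TDS_Character owner, with sound and AI noise on each shot.
; A trigger press opens a Gate that re-enters itself every 0.1 seconds while consuming ammo; release only calls the parent, never closing it.
; Reloading recalculates clip and reserve ammo, animates ammo widgets, and sets a flag blocking new presses until a delay clears it.
; The double-gun spawn logic is unconnected.
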(event EventBeginPlay
  (|CallParentFunction) ; This node is disabled and will not be called.\nDrag off pins to build functionality.
)

(event Collision|EventActorBeginOverlap
  (params (OtherActor :type Actor%20Object%20Reference))
  (|CallParentFunction OtherActor) ; This node is disabled and will not be called.\nDrag off pins to build functionality.
)

(event EventTick
  (params (DeltaSeconds :type Float%20%28single-precision%29)))

(event EventTriggerPressed
  (bind _muzzle_ref (Variables|Default|GetMuzzle%20Ref))
  (bind _returnvalue (Transformation|GetWorldRotation _muzzle_ref))
  (|CallParentFunction)
  (if (not (Variables|Default|GetReload))
    (bind _asbp_tds_character (Utilities|Casting|CastToBP_TDS_Character (Variables|Default|GetGunOwner)))
    (if (Variables|/Game/MyContent/Blueprints/Characters/BP_TDS_Character.BP_TDS_Character_C|GetUseGun _asbp_tds_character)
      (Utilities|FlowControl|Sequence
        (:then_0
          (goto _label Open))
        (:then_1
          (Utilities|FlowControl|Gate true :!label _label
            (:Exit
              (Utilities|FlowControl|Sequence
                (:then_0
                  (Utilities|FlowControl|RetriggerableDelay 0.1)
                  (goto _label))
                (:then_1
                  (if (>= (Variables|Default|GetGunAmmo) 1)
                    (Variables|Default|SetGunAmmo (- (Variables|Default|GetGunAmmo) 1))
                    (Game|SpawnActorfromClass "/Game/MyContent/Blueprints/Projectiles/BP_CharacterProjectile.BP_CharacterProjectile_C" (Math|Transform|MakeTransform (+ (Transformation|GetWorldLocation (Variables|Default|GetMuzzle%20Ref)) (Math|Vector|GetForwardVector _returnvalue)) _returnvalue "0.050000,0.050000,0.050000") "AlwaysSpawn" (Variables|Default|GetGunOwner) 5.0 0)
                    (Audio|PlaySoundatLocation (Variables|Default|GetShootSFX) (Transformation|GetActorLocation) "0, 0, 0" 1.0 1.0 0.0 0 0 0) ; Play firing sound
                    (bind _asbp_tds_character_2 (Utilities|Casting|CastToBP_TDS_Character (Variables|Default|GetGunOwner)))
                    (Class|PawnNoiseEmitterComponent|MakeNoise (Variables|/Game/MyContent/Blueprints/Characters/BP_TDS_Character.BP_TDS_Character_C|GetPawnNoiseEmitter _asbp_tds_character_2) self 1.0 (Transformation|GetActorLocation))))))))))))

(event EventReloading
  (|CallParentFunction)
  (bind _asbp_tds_character (Utilities|Casting|CastToBP_TDS_Character (Variables|Default|GetGunOwner)))
  (if (Variables|/Game/MyContent/Blueprints/Characters/BP_TDS_Character.BP_TDS_Character_C|GetUseGun _asbp_tds_character)
    (if (>= (Variables|Default|GetGunAmmo) 1)
      (Variables|Default|SetNeedAmmo (- (Variables|Default|GetAmmoClip) (Variables|Default|GetGunAmmo)))
      (if (<= (Variables|Default|GetGunAmmo) (Variables|Default|GetNeedAmmo))
        (Variables|Default|SetGunAmmo (+ (Variables|Default|GetGunAmmo) (Variables|Default|GetGunAmmoMax)))
        (Variables|Default|SetGunAmmoMax 0)
        (else
          (Variables|Default|SetGunAmmoMax (- (Variables|Default|GetGunAmmo) (Variables|Default|GetNeedAmmo)))
          (Variables|Default|SetGunAmmo 30)))
      (Variables|Default|SetReload true)
      (Audio|Components|Audio|Play (Variables|Default|GetReloadSFX) 0.0)
      (bind _foundwidgets (Widget|GetAllWidgetsOfClass "/Game/MyContent/Widgets/BP_GunAmmoWidget.BP_GunAmmoWidget_C" false))
      (for _array_element _foundwidgets
        (Class|UserWidget|PlayAnimationForward _array_element (Variables|/Game/MyContent/Widgets/BP_GunAmmoWidget.BP_GunAmmoWidget_C|GetButtonAnim _array_element) 1.0 false)
        (Class|UserWidget|PlayAnimationForward _array_element (Variables|/Game/MyContent/Widgets/BP_GunAmmoWidget.BP_GunAmmoWidget_C|GetTextAnim _array_element) 1.0 false)
        (Class|UserWidget|PlayAnimationForward _array_element (Variables|/Game/MyContent/Widgets/BP_GunAmmoWidget.BP_GunAmmoWidget_C|GetTextAnimation _array_element) 1.0 false)
        (Utilities|FlowControl|Delay 1.0)
        (Variables|Default|SetReload false)))))

(event EventTriggerReleased
  (|CallParentFunction))

(fn ConstructionScript
  (|CallParentFunction))