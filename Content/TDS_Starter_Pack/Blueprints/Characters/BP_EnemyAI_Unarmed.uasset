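; Unarmed enemy AI character that turns toward the player and closes in for a melee attack.
; Attack, skipped when dead, yaws the enemy to face the player, then uses AI MoveTo if Distance is within a fixed range, or calls SearchCharacter otherwise.
; A successful move triggers Melee, which is only a placeholder debug print.
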(event Custom|Melee
  (Development|PrintString "Melee Attack"))

(event EventBeginPlay
  (|CallParentFunction) ; This node is disabled and will not be called.\nDrag off pins to build functionality.
)

(event Collision|EventActorBeginOverlap
  (params (OtherActor :type Actor%20Object%20Reference)))

(event EventTick
  (params (DeltaSeconds :type Float%20%28single-precision%29))
  (|CallParentFunction DeltaSeconds) ; This node is disabled and will not be called.\nDrag off pins to build functionality.
)

(event EventAttack
  (bind _asbp_tds_character (Utilities|Casting|CastToBP_TDS_Character (Game|GetPlayerCharacter 0)))
  (Variables|Default|SetShooterCharacter _asbp_tds_character)
  (if (not (Variables|Default|GetDeath))
    (Variables|Default|SetAttack? true)
    (Transformation|SetActorRotation (Math|Rotator|MakeRotator 0.0 0.0 (.Yaw (Math|Rotator|BreakRotator (Math|Rotator|FindLookatRotation (Transformation|GetActorLocation) (Transformation|GetActorLocation _asbp_tds_character))))))
    (if (<= (Variables|Default|GetDistance) 5e+02)
      (AI|AIMoveTo self "0, 0, 0" (Variables|Default|GetShooterCharacter) 25.0 false
        (:OnSuccess
          (CallFunction|Melee)))
      (else
        (CallFunction|SearchCharacter)))))

(fn ConstructionScript
  (|CallParentFunction))