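; Master enemy AI for a top-down shooter: detects the player and sedans, searches via AIMoveTo, and flees fast cars.
; It shoots projectiles at slow occupied cars and reloads, but the player-attack, damage FX and flashlight events are empty, their logic disconnected.
; Damage turns it toward the player.
; Tick-polled death plays a random animation or ragdolls after car hits; other kills award XP and sometimes trigger a slow-motion camera blend.
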(event OnComponentBeginOverlap(Capsule)
  (params (OverlappedComponent :type Primitive%20Component%20Object%20Reference) (OtherActor :type Actor%20Object%20Reference) (OtherComp :type Primitive%20Component%20Object%20Reference) (OtherBodyIndex :type Integer) (bFromSweep :type Boolean) (SweepResult :type Hit%20Result%20Structure%20%28by%20ref%29))
  ;[1 1 1] Car Hit Event
  (bind _asbp_sedan (Utilities|Casting|CastToBP_Sedan OtherActor))
  (Utilities|IsValid (Variables|/Script/PhysXVehicles.WheeledVehicle|GetVehicleMovement _asbp_sedan)
    (:Is%20Valid
      (if (or (>= (Class|WheeledVehicleMovementComponent|GetForwardSpeed (Variables|/Script/PhysXVehicles.WheeledVehicle|GetVehicleMovement _asbp_sedan)) 5e+02) (<= (Class|WheeledVehicleMovementComponent|GetForwardSpeed (Variables|/Script/PhysXVehicles.WheeledVehicle|GetVehicleMovement _asbp_sedan)) -5e+02))
        (Variables|Default|SetHealth 0.0)
        (Variables|Default|SetDeathByCar true)
        (Audio|Components|Audio|Play (Variables|Default|GetHit) 0.0)))))

(event OnSeePawn(PawnSensing)
  (params (Pawn :type Pawn%20Object%20Reference))
  ;[1 1 1] When an enemy sees, or hears, a player, he will attack him. If he saw, or heard the enemy, but lost him from sight, then the enemy, after a pause, begins to look for a player
  (bind _asbp_tds_character (Utilities|Casting|CastToBP_TDS_Character Pawn))
  (if (not (Variables|/Game/TDS_Starter_Pack/Blueprints/Characters/BP_TDS_Character.BP_TDS_Character_C|GetDead _asbp_tds_character))
    (if (not (Variables|Default|GetDeath))
      (Variables|Default|SetInRange true)
      (Variables|Default|SetSeePlayer true)
      (CallFunction|Attack)
      (Utilities|FlowControl|Delay 1.0)
      (Variables|Default|SetInRange false)
      (if (Variables|Default|GetSeePlayer)
        (Utilities|FlowControl|Delay 5.0)
        (if (not (Variables|Default|GetInRange))
          (CallFunction|SearchCharacter))))))

(event OnHearNoise(PawnSensing)
  (params (Instigator :type Pawn%20Object%20Reference) (Location :type Vector%20%28by%20ref%29 :default "0, 0, 0") (Volume :type Float%20%28single-precision%29))
  ;[1 1 1] When an enemy sees, or hears, a player, he will attack him. If he saw, or heard the enemy, but lost him from sight, then the enemy, after a pause, begins to look for a player
  (if (not (Variables|Default|GetDeath))
    (Variables|Default|SetInRange true)
    (Variables|Default|SetSeePlayer true)
    (CallFunction|Attack)
    (Utilities|FlowControl|Delay 1.0)
    (Variables|Default|SetInRange false)
    (if (Variables|Default|GetSeePlayer)
      (Utilities|FlowControl|Delay 5.0)
      (if (not (Variables|Default|GetInRange))
        (CallFunction|SearchCharacter)))))

(event OnSeePawn(PawnSensing1)
  (params (Pawn :type Pawn%20Object%20Reference))
  ;[1 1 1] If a car with a character inside moves fast, the enemy escapes to a random point. Upon reaching it, he returns to the initial location.
  (bind _asbp_sedan (Utilities|Casting|CastToBP_Sedan Pawn))
  (Utilities|IsValid (Variables|/Script/PhysXVehicles.WheeledVehicle|GetVehicleMovement _asbp_sedan)
    (:Is%20Valid
      (if (or (>= (Class|WheeledVehicleMovementComponent|GetForwardSpeed (Variables|/Script/PhysXVehicles.WheeledVehicle|GetVehicleMovement _asbp_sedan)) 5e+02) (<= (Class|WheeledVehicleMovementComponent|GetForwardSpeed (Variables|/Script/PhysXVehicles.WheeledVehicle|GetVehicleMovement _asbp_sedan)) -5e+02))
        (AI|AIMoveTo self (.RandomLocation (Class|NavigationSystemV1|GetRandomPointinNavigableRadius (Transformation|GetActorLocation _asbp_sedan) 6e+03 0 0)) 0 5.0 false
          (:OnSuccess
            (Utilities|FlowControl|Delay 3.0)
            (AI|AIMoveTo self (Variables|Default|GetInitialLocation) 0 5.0 false)))
        (elif (Variables|/Game/TDS_Starter_Pack/Blueprints/Vehicles/BP_Sedan.BP_Sedan_C|GetInCar _asbp_sedan)
          (CallFunction|AttackCar))))))

(event Custom|DeathEvent
  (bind _deathanimseqs (Variables|Default|GetDeathAnimSeqs))
  (bind _shootercharacter (Variables|Default|GetShooterCharacter))
  (bind _capsule (Variables|Default|GetCapsule))
  ;[1 1 1] if health is zero or less, the “Dead” variable becomes true, animation plays, components are destroyed, other components are given a static type of collision so that they can no longer be shot at.
  (if (<= (Variables|Default|GetHealth) 0.0)
    (Variables|Default|SetDeath true)
    (Utilities|FlowControl|DoOnce false
      (:Completed
        (Components|Animation|PlayAnimation (Variables|Character|GetMesh) (Utilities|Array|Get(acopy) _deathanimseqs (Math|Random|RandomIntegerinRange 0 (- (Utilities|Array|Length _deathanimseqs) 1))) false)
        (Components|DestroyComponent (Variables|Character|GetCharacterMovement))
        (Collision|SetCollisionObjectType (Variables|Collision|GetCapsuleComponent) "ECC_WorldStatic")
        (Utilities|IsValid _capsule
          (:Is%20Valid
            (Components|DestroyComponent _capsule)
            (if (Variables|Default|GetDeathByCar)
              (Physics|SetSimulatePhysics (Variables|Character|GetMesh) true)
              (else
                ;;[1 1 1] WhenCharacterKillTheEnemies - + XP
                (Utilities|IsValid _shootercharacter
                  (:Is%20Valid
                    (Variables|/Game/TDS_Starter_Pack/Blueprints/Characters/BP_TDS_Character.BP_TDS_Character_C|SetXP _shootercharacter (+ (Variables|/Game/TDS_Starter_Pack/Blueprints/Characters/BP_TDS_Character.BP_TDS_Character_C|GetXP _shootercharacter) 100))
                    (bind _foundwidgets (Widget|GetAllWidgetsOfClass "/Game/TDS_Starter_Pack/Widgets/BP_HUD_Widget.BP_HUD_Widget_C" false))
                    (for _array_element _foundwidgets
                      (UserInterface|Animation|PlayAnimation _array_element (Variables|/Game/TDS_Starter_Pack/Widgets/BP_HUD_Widget.BP_HUD_Widget_C|GetXP_TextAnim _array_element) 0.0 1 "Forward" 1.0 false)
                      ;;[1 1 1] SlowMoEvent
                      (if (== (Math|Random|RandomIntegerinRange 0 4) 4)
                        (Variables|Default|SetSlowMo true)
                        (Utilities|Time|SetGlobalTimeDilation 0.1)
                        (Audio|Components|Audio|Play (Variables|Default|Getaiming_reverse_wav_Cue) 0.0)
                        (Game|Player|SetViewTargetwithBlend (Game|GetPlayerController 0) self 0.1 "VTBlend_Linear" 0.0 false)
                        (Utilities|FlowControl|Delay 0.2)
                        (Game|Player|SetViewTargetwithBlend (Game|GetPlayerController 0) (Game|GetPlayerCharacter 0) 0.1 "VTBlend_Linear" 0.0 false)
                        (Audio|Components|Audio|Play (Variables|Default|Getreverese_Cue) 0.0)
                        (Utilities|Time|SetGlobalTimeDilation 1.0)
                        (Audio|Components|Audio|SetPitchMultiplier (Variables|Default|GetAttackAudio) 1.0)
                        (for _array_element_2 0
                          (Audio|Components|Audio|SetPitchMultiplier (Variables|/Script/Engine.AmbientSound|GetAudioComponent _array_element_2) 1.0)
                          (Variables|Default|SetSlowMo false))))))))))))))

(event Custom|Attack
  ;[1 1 1] If the enemy sees the player and is not dead, does not recharge, then he will attack the player if the distance is less than 500 units. If there are no ammo it is recharged.
)

(event Custom|Reload
  ;[1 1 1] Reloading
  (if (< (Variables|Default|GetAmmo) 8)
    (if (not (Variables|Default|GetDeath))
      (Components|Animation|PlayAnimation (Variables|Character|GetMesh) "/Game/TDS_Starter_Pack/ExampleContent/AnimStarterPack/Reload_Shotgun_Hip.Reload_Shotgun_Hip" false)
      (Variables|Default|SetReloading true)
      (if (>= (Variables|Default|GetMaxAmmo) 0)
        (Variables|Default|SetNeedAmmo (- (Variables|Default|GetMaxAmmo) 8))
        (if (<= (Variables|Default|GetMaxAmmo) (Variables|Default|GetNeedAmmo))
          (Variables|Default|SetAmmo (+ (Variables|Default|GetAmmo) (Variables|Default|GetMaxAmmo)))
          (Variables|Default|SetMaxAmmo 0)
          (else
            (Variables|Default|SetMaxAmmo (- (Variables|Default|GetMaxAmmo) (Variables|Default|GetNeedAmmo)))
            (Variables|Default|SetAmmo 8)))
        (Utilities|FlowControl|Delay 4.3)
        (Variables|Default|SetReloading false)
        (if (not (Variables|Default|GetDeath))
          (Components|Animation|SetAnimationMode (Variables|Character|GetMesh) "AnimationBlueprint"))))))

(event Custom|Night?
  ;[1 1 1] IfNightTrue - Flashlight On
)

(event Custom|SearchCharacter
  (bind _returnvalue (Game|GetPlayerCharacter 0))
  ;[1 1 1] Player search. With success = attack.
  (if (not (Variables|Default|GetDeath))
    (if (not (Variables|Default|GetReloading))
      (Utilities|IsValid _returnvalue
        (:Is%20Valid
          (Variables|Default|SetDistance (Math|Vector|VectorLength (- (Transformation|GetActorLocation) (Transformation|GetActorLocation _returnvalue))))
          (AI|AIMoveTo self (+ (Transformation|GetActorLocation) "500.000000,500.000000,0.000000") (Variables|Default|GetShooterCharacter) 5.0 false
            (:then
              (if (<= (Variables|Default|GetDistance) 5e+02)
                (CallFunction|Attack)))))))))

(event Custom|ApplyDamgeFX
  ;[1 1 1] Apply Damage FX
)

(event Custom|AttackCar
  (bind _arrow1 (Variables|Default|GetArrow1))
  (bind _returnvalue (Transformation|GetWorldRotation _arrow1))
  ;[1 1 1] If the car is standing with the character inside or moving slowly, the enemy attacks the car, causing damage to it.
  (if (not (Variables|Default|GetDeath))
    (if (not (Variables|Default|GetReloading))
      (Variables|Default|SetAttack? true)
      (Components|Movement|StopMovementImmediately (Variables|Character|GetCharacterMovement))
      (Transformation|SetActorRotation (Math|Rotator|MakeRotator 0.0 0.0 (.Yaw (Math|Rotator|BreakRotator (Math|Rotator|FindLookatRotation (Transformation|GetActorLocation) (Transformation|GetActorLocation (stale OnSeePawn(PawnSensing1) _asbp_sedan)))))))
      (if (<= (Variables|Default|GetDistance) 5e+02)
        (if (>= (Variables|Default|GetAmmo) 1)
          (Variables|Default|SetAmmo (- (Variables|Default|GetAmmo) 1))
          (Game|SpawnActorfromClass "/Game/TDS_Starter_Pack/Blueprints/Projectiles/BP_EnemyProjectile.BP_EnemyProjectile_C" (Math|Transform|MakeTransform (+ (Transformation|GetWorldLocation (Variables|Default|GetArrow1)) (Math|Vector|RotateVector (Variables|Default|GetGunOfset) _returnvalue)) _returnvalue) "Undefined" 0 0)
          (Audio|Components|Audio|Play (Variables|Default|GetAttackAudio) 0.0)
          (else
            (CallFunction|Reload)))
        (else
          (CallFunction|SearchCharacter))))))

(event Game|Damage|EventAnyDamage
  (params (Damage :type Float%20%28single-precision%29) (DamageType :type Damage%20Type%20Object%20Reference) (InstigatedBy :type Controller%20Object%20Reference) (DamageCauser :type Actor%20Object%20Reference))
  ;[1 1 1] When receiving damage the enemy loses health corresponding to damage.
  (Variables|Default|SetHealth (- (Variables|Default|GetHealth) Damage))
  (Transformation|SetActorRotation (Math|Rotator|MakeRotator 0.0 0.0 (.Yaw (Math|Rotator|BreakRotator (Math|Rotator|FindLookatRotation (Transformation|GetActorLocation) (Transformation|GetActorLocation (Variables|Default|GetShooterCharacter)))))))
  (CallFunction|ApplyDamgeFX))

(event EventTick
  (params (DeltaSeconds :type Float%20%28single-precision%29))
  ;[1 1 1] Event Tick Cheking Death of Enemy
  (CallFunction|DeathEvent))

(event EventBeginPlay
  ;[1 1 1] Event Begin Play\set Initial Location/if night - turn on flashlight
  (bind _asbp_tds_character (Utilities|Casting|CastToBP_TDS_Character (Game|GetPlayerCharacter 0)))
  (Variables|Default|SetShooterCharacter _asbp_tds_character)
  (Variables|Default|SetInitialLocation (Transformation|GetActorLocation))
  (Utilities|FlowControl|Delay 0.2)
  (CallFunction|Night?))

(fn ConstructionScript)