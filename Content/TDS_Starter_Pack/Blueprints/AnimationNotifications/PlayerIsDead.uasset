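; Animation notify, named for the player's death, that sets nearby enemy creatures to their eating state.
; When it fires, it sphere-overlaps pawns around the animated mesh's location, filtering for BP_EnemyAI_Creature and ignoring the player character.
; Each creature found gets its Eating flag set, and its display name is printed as debug output.
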(fn GetNotifyName
  (return (Variables|Default|GetNotificationName)))

(fn ReceivedNotify
  (params (MeshComp :type Skeletal%20Mesh%20Component%20Object%20Reference) (Animation :type Anim%20Sequence%20Base%20Object%20Reference))
  (bind _outactors (Collision|SphereOverlapActors (Transformation|GetWorldLocation MeshComp) 1e+03 (Utilities|Array|MakeArray "ObjectTypeQuery3") "/Game/TDS_Starter_Pack/Blueprints/Characters/BP_EnemyAI_Creature.BP_EnemyAI_Creature_C" (Utilities|Array|MakeArray (Game|GetPlayerCharacter 0))))
  (for _array_element _outactors
    (bind _asbp_enemy_ai_creature (Utilities|Casting|CastToBP_EnemyAI_Creature _array_element))
    (Variables|/Game/TDS_Starter_Pack/Blueprints/Characters/BP_EnemyAI_Creature.BP_EnemyAI_Creature_C|SetEating _asbp_enemy_ai_creature true)
    (Development|PrintString (Utilities|String|ToString(Text) (Utilities|Text|FormatText (Utilities|Text|ToText(String) (Utilities|GetDisplayName _asbp_enemy_ai_creature))))))
  (return false))