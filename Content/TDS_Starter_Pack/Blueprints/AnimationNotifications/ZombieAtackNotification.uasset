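; Anim notify for the zombie attack animation that damages the player when the strike lands.
; When triggered, it checks whether player 0 is within AttackDistance of the mesh owner in 2D, ignoring height, with no trace or facing check.
; On a hit, it applies fixed damage, attaches a random blood emitter to the player's mesh and spawns a blood splatter decal at the player's location.
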(fn GetNotifyName
  (return (Variables|Default|GetNotificatioName)))

(fn ReceivedNotify
  (params (MeshComp :type Skeletal%20Mesh%20Component%20Object%20Reference) (Animation :type Anim%20Sequence%20Base%20Object%20Reference))
  (bind _emitter_template (Variables|Default|GetEmitter%20Template))
  (LocalVariables|SetOwner (Components|GetOwner MeshComp))
  (LocalVariables|SetPlayerCharacter (Game|GetPlayerCharacter 0))
  (if (< (Math|Vector|Distance2D(Vector) (Transformation|GetActorLocation (LocalVariables|GetOwner)) (Transformation|GetActorLocation (LocalVariables|GetPlayerCharacter))) (Variables|Default|GetAttackDistance))
    (Game|Damage|ApplyDamage (LocalVariables|GetPlayerCharacter) 5e+01 0 (LocalVariables|GetOwner) "/Script/Engine.DamageType")
    ;[1 1 1] Apply Blood Effects
    (bind _returnvalue (Effects|SpawnEmitterAttached (Utilities|Array|Get(acopy) _emitter_template (Math|Random|RandomIntegerinRange 0 (Utilities|Array|Length _emitter_template))) (Variables|/Script/Engine.Character|GetMesh (LocalVariables|GetPlayerCharacter)) "None" "0, 0, 0" "0, 0, 0" "2.000000,2.000000,2.000000" "SnapToTarget" true "AutoRelease"))
    (LocalVariables|SetlBloodEmitter _returnvalue)
    (bind _returnvalue_2 (Rendering|Decal|SpawnDecalatLocation "/Game/BallisticsVFX/Decals/Splashers/Decal_Blood_Splatter.Decal_Blood_Splatter" "250.000000,250.000000,250.000000" (Transformation|GetActorLocation (LocalVariables|GetPlayerCharacter)) "-90.000000,0.000000,0.000000" 0.0))
    (LocalVariables|SetlBloodDecal _returnvalue_2)
    (return (< (Math|Vector|Distance2D(Vector) (Transformation|GetActorLocation (LocalVariables|GetOwner)) (Transformation|GetActorLocation (LocalVariables|GetPlayerCharacter))) (Variables|Default|GetAttackDistance)))))