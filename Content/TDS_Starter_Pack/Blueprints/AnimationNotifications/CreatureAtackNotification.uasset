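; Animation notify that lets a creature's attack animation damage the player.
; When it fires, it measures the 2D distance between the mesh's owner and player character 0.
; If that is below the attack distance, it applies fixed base damage of the configured damage type, with the owner as causer.
; The notify's display name comes from a variable.
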(fn GetNotifyName
  (return (Variables|Default|GetNotificatioName)))

(fn ReceivedNotify
  (params (MeshComp :type Skeletal%20Mesh%20Component%20Object%20Reference) (Animation :type Anim%20Sequence%20Base%20Object%20Reference))
  (LocalVariables|SetOwner (Components|GetOwner MeshComp))
  (LocalVariables|SetPlayerCharacter (Game|GetPlayerCharacter 0))
  (if (< (Math|Vector|Distance2D(Vector) (Transformation|GetActorLocation (LocalVariables|GetOwner)) (Transformation|GetActorLocation (LocalVariables|GetPlayerCharacter))) (Variables|Default|GetAttackDistance))
    (Game|Damage|ApplyDamage (LocalVariables|GetPlayerCharacter) 5e+01 0 (LocalVariables|GetOwner) "/Script/Engine.DamageType")
    (return (< (Math|Vector|Distance2D(Vector) (Transformation|GetActorLocation (LocalVariables|GetOwner)) (Transformation|GetActorLocation (LocalVariables|GetPlayerCharacter))) (Variables|Default|GetAttackDistance)))))